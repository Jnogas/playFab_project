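; Checkpoint actor for a 3D platformer that registers itself as the player's latest checkpoint when touched.
; An overlap on its CheckPointRadius component by a BP_ThirdPersonCharacter stores the actor in that character's LatestCheckPoint.
; It then spawns a particle system at ParticleLocation and plays a sound.
; A CheckpointFlagged boolean and a DoOnce limit activation to a single time.
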(event `self.CheckPointRadius.OnComponentBeginOverlap`
  (params (OverlappedComponent :type "PrimitiveComponent Object Reference") (OtherActor :type "Actor Object Reference") (OtherComp :type "PrimitiveComponent Object Reference") (OtherBodyIndex :type Integer) (bFromSweep :type Boolean) (SweepResult :type "HitResult Structure (by ref)"))
  (if (not (`self.CheckpointFlagged`))
    (bind _asbp_third_person_character (cast `/Game/Easy3DPlatformerKit/Demo/ThirdPerson/BluePrints/BP_ThirdPersonCharacter` OtherActor))
    (`/Engine/EditorBlueprintResources/StandardMacros.DoOnce` false
      (:`Completed`
        (set `/Game/Easy3DPlatformerKit/Demo/ThirdPerson/BluePrints/BP_ThirdPersonCharacter.LatestCheckPoint` self _asbp_third_person_character)
        (set `self.CheckpointFlagged` true)
        (`NiagaraFunctionLibrary.SpawnSystemAtLocation` "/Game/Easy3DPlatformerKit/Demo/Particles/NS_Checkpoint.NS_Checkpoint" (`SceneComponent.K2_GetComponentLocation` (`self.ParticleLocation`)))
        (`GameplayStatics.PlaySoundAtLocation` "/Game/Easy3DPlatformerKit/Main/Audio/WAV/AU_Checkpoint.AU_Checkpoint" (`self.K2_GetActorLocation`) (struct) 1.0 1.0 0.0 null null null null)))))

(fn `UserConstructionScript`)