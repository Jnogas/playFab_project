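; BP_LevelFinish is the level-end checkpoint that sends the player on to the next level.
; When a BP_ThirdPersonCharacter overlaps CheckPointRadius, a DoOnce gate fires a finish sound, a Niagara effect at ParticleLocation, and the WD_FinishLevel widget.
; After the WaitTimeForNextLevel delay, it removes the widget and opens the level named in NextLevelName.
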(event `self.CheckPointRadius.OnComponentBeginOverlap`
  (params (OverlappedComponent :type "PrimitiveComponent Object Reference") (OtherActor :type "Actor Object Reference") (OtherComp :type "PrimitiveComponent Object Reference") (OtherBodyIndex :type Integer) (bFromSweep :type Boolean) (SweepResult :type "HitResult Structure (by ref)"))
  (cast `/Game/Easy3DPlatformerKit/Demo/ThirdPerson/BluePrints/BP_ThirdPersonCharacter` OtherActor)
  (`/Engine/EditorBlueprintResources/StandardMacros.DoOnce` false
    (:`Completed`
      (`GameplayStatics.PlaySound2D` "/Game/Easy3DPlatformerKit/Main/Audio/WAV/AU_FinishLevel.AU_FinishLevel" 1.0 1.0 0.0 null null)
      (`NiagaraFunctionLibrary.SpawnSystemAtLocation` "/Game/Easy3DPlatformerKit/Demo/Particles/NS_Checkpoint.NS_Checkpoint" (`SceneComponent.K2_GetComponentLocation` (`self.ParticleLocation`)))
      (bind _returnvalue (`|CreateWidget` "/Game/Easy3DPlatformerKit/Main/Widgets/WD_FinishLevel.WD_FinishLevel_C"))
      (bind _output_get (set `self.FinishLevelWidget` _returnvalue))
      (`UserWidget.AddToViewport` _output_get 0)
      (`KismetSystemLibrary.Delay` (`self.WaitTimeForNextLevel`))
      (`Widget.RemoveFromParent` (`self.FinishLevelWidget`))
      (`GameplayStatics.OpenLevel` (`self.Next Level Name`)))))

(fn `UserConstructionScript`)