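; Turret AI that aims at and shoots the third-person player character when its PawnSensing component sees it.
; BeginPlay sets the sight radius from TurretRange.
; Each sighting turns TurretSides by yaw and TurretMain by pitch, using a look-at rotation toward the player.
; A one-second Delay, which ignores retriggers while pending, paces the BP_Bullet spawns at ParticleLocation and the firing sound.
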(event `self.ReceiveBeginPlay`
  (set `PawnSensingComponent.SightRadius` (`self.TurretRange`) (`self.PawnSensing`)))

(event `self.PawnSensing.OnSeePawn`
  (params (Pawn :type "Pawn Object Reference"))
  (bind (_returnvalue_roll _returnvalue_pitch _returnvalue_yaw) (`KismetMathLibrary.BreakRotator` (`SceneComponent.K2_GetComponentRotation` (`self.TurretSides`))))
  (bind (_returnvalue_location _returnvalue_rotation) (`KismetMathLibrary.BreakTransform` (`SceneComponent.K2_GetComponentToWorld` (`self.ParticleLocation`))))
  (bind _asbp_third_person_character (cast `/Game/Easy3DPlatformerKit/Demo/ThirdPerson/BluePrints/BP_ThirdPersonCharacter` Pawn))
  (`|ExecutionSequence`
    (:`then_0`
      (bind (_returnvalue_roll_2 _returnvalue_pitch_2 _returnvalue_yaw_2) (`KismetMathLibrary.BreakRotator` (`KismetMathLibrary.FindLookAtRotation` (`self.K2_GetActorLocation`) (`self.K2_GetActorLocation` _asbp_third_person_character))))
      (`SceneComponent.K2_SetWorldRotation` (`self.TurretSides`) (`KismetMathLibrary.MakeRotator` 0.0 0.0 _returnvalue_yaw_2) false false)
      (`SceneComponent.K2_SetWorldRotation` (`self.TurretMain`) (`KismetMathLibrary.MakeRotator` 0.0 _returnvalue_pitch_2 _returnvalue_yaw) false false))
    (:`then_1`
      (`KismetSystemLibrary.Delay` 1.0)
      (`|SpawnActorFromClass` "/Game/Easy3DPlatformerKit/Main/Blueprints/Turret/BP_Bullet.BP_Bullet_C" (`KismetMathLibrary.MakeTransform` _returnvalue_location _returnvalue_rotation) "Undefined" "OverrideRootScale" null null)
      (`GameplayStatics.PlaySoundAtLocation` "/Game/Easy3DPlatformerKit/Main/Audio/WAV/AU_Turret.AU_Turret" (`self.K2_GetActorLocation`) (struct) 1.0 1.0 0.0 null null null null))))

(fn `UserConstructionScript`)