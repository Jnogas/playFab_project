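; A platform that falls away shortly after the third-person character steps on it, then respawns.
; An overlap on its box trigger starts a DoOnce-guarded sequence that swaps the cube through two warning materials over PlatformFallTime.
; The platform then hides and loses collision rather than physically moving.
; After a fixed delay it restores its material, collision and visibility and rearms the trigger.
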(event `self.Box.OnComponentBeginOverlap`
  (params (OverlappedComponent :type "PrimitiveComponent Object Reference") (OtherActor :type "Actor Object Reference") (OtherComp :type "PrimitiveComponent Object Reference") (OtherBodyIndex :type Integer) (bFromSweep :type Boolean) (SweepResult :type "HitResult Structure (by ref)"))
  (bind _cube (`self.Cube`))
  (cast `/Game/Easy3DPlatformerKit/Demo/ThirdPerson/BluePrints/BP_ThirdPersonCharacter` OtherActor)
  (`/Engine/EditorBlueprintResources/StandardMacros.DoOnce` false :!label _label
    (:`Completed`
      (`PrimitiveComponent.SetMaterial` (`self.Cube`) 0 "/Game/Easy3DPlatformerKit/Demo/Materials/M_FallingPlatform_Stage_1.M_FallingPlatform_Stage_1")
      (`KismetSystemLibrary.Delay` (/ (`self.PlatformFallTime`) 2.0))
      (`PrimitiveComponent.SetMaterial` (`self.Cube`) 0 "/Game/Easy3DPlatformerKit/Demo/Materials/M_FallingPlatform_Stage_2.M_FallingPlatform_Stage_2")
      (`KismetSystemLibrary.Delay` (/ (`self.PlatformFallTime`) 2.0))
      (`SceneComponent.SetVisibility` (`self.DefaultSceneRoot`) false true)
      (`PrimitiveComponent.SetCollisionEnabled` (`self.Cube`) "NoCollision")
      (`KismetSystemLibrary.Delay` 3.0)
      (`PrimitiveComponent.SetMaterial` _cube 0 "/Game/Easy3DPlatformerKit/Demo/Materials/M_Platform.M_Platform")
      (`PrimitiveComponent.SetCollisionEnabled` _cube "QueryAndPhysics")
      (`SceneComponent.SetVisibility` (`self.DefaultSceneRoot`) true true)
      (goto _label :!via `Reset`))))

(fn `UserConstructionScript`)